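; BP_ExplosionGrid is a trigger actor that launches a BP_Wheelchair with an explosion effect when it overlaps the box.
; The overlap applies a velocity-change impulse to the wheelchair mesh, upward and along a world axis chosen by the Directions setting and scaled by Force.
; A particle system spawned at BeginPlay is activated briefly, while the scene component hides and box collision switches off until both restore after a cooldown.
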(event `self.ReceiveBeginPlay`
  (bind _returnvalue (`GameplayStatics.SpawnEmitterAtLocation` "/Engine/Tutorial/SubEditors/TutorialAssets/TutorialParticleSystem.TutorialParticleSystem" (`self.K2_GetActorLocation`) (struct) (15.0 15.0 50.0) false))
  (bind _output_get (set `self.ExplosionParticle` _returnvalue))
  (`ActorComponent.Deactivate` _output_get))

(event `self.Box.OnComponentBeginOverlap`
  (params (OverlappedComponent :type "PrimitiveComponent Object Reference") (OtherActor :type "Actor Object Reference") (OtherComp :type "PrimitiveComponent Object Reference") (OtherBodyIndex :type Integer) (bFromSweep :type Boolean) (SweepResult :type "HitResult Structure (by ref)"))
  (bind _explosionparticle (`self.ExplosionParticle`))
  (bind _force (`self.Force`))
  (bind _returnvalue (* _force -1.0))
  (bind _asbp_wheelchair (cast `/Game/Blueprints/Actors/BP_Wheelchair` OtherActor))
  (`PrimitiveComponent.AddImpulse` (`/Game/Blueprints/Actors/BP_Wheelchair.StaticMesh` _asbp_wheelchair) (select `/Game/ENUM/EN_Directions` (`self.Directions`) :`NewEnumerator0` (`KismetMathLibrary.MakeVector` _force 0.0 _force) :`NewEnumerator1` (`KismetMathLibrary.MakeVector` _returnvalue 0.0 _force) :`NewEnumerator2` (`KismetMathLibrary.MakeVector` 0.0 _force _force) :`NewEnumerator3` (`KismetMathLibrary.MakeVector` 0.0 _returnvalue _force) :!type "Vector Structure") "None" true)
  (`|ExecutionSequence`
    (:`then_0`
      (`ActorComponent.Activate` _explosionparticle false)
      (`KismetSystemLibrary.RetriggerableDelay` 2.0)
      (`ActorComponent.Deactivate` _explosionparticle))
    (:`then_1`
      (`SceneComponent.SetVisibility` (`self.Scene`) false true)
      (`PrimitiveComponent.SetCollisionEnabled` (`self.Box`) "NoCollision")
      (`KismetSystemLibrary.Delay` 10.0)
      (`SceneComponent.SetVisibility` (`self.Scene`) true true)
      (`PrimitiveComponent.SetCollisionEnabled` (`self.Box`) "QueryAndPhysics"))))

(fn `UserConstructionScript`)