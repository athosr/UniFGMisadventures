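; BP_Turnstile is an actor whose point light flickers during play.
; BeginPlay starts the Flickering event, which waits a short random delay, shows the light, waits a longer random delay, then hides it.
; The event then calls itself, so the irregular on-off cycle repeats indefinitely.
; The graphs contain no turnstile movement or interaction logic, and the construction script is empty.
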(event `self.ReceiveBeginPlay`
  (`self.Flickering`))

(event `Flickering`
  (`KismetSystemLibrary.Delay` (`KismetMathLibrary.RandomFloatInRange` 0.5 1.5))
  (`SceneComponent.SetVisibility` (`self.PointLight`) true false)
  (`KismetSystemLibrary.Delay` (`KismetMathLibrary.RandomFloatInRange` 1.0 3.0))
  (`SceneComponent.SetVisibility` (`self.PointLight`) false false)
  (`self.Flickering`))

(fn `UserConstructionScript`)