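; BP_Wheelchair is a player-driven, physics-based wheelchair that moves on four hover components bound to its static mesh.
; Forward input adds acceleration along the mesh's forward vector while any hover component reports CanMove, and a constant downward force applies every tick.
; Turn input applies yaw torque ungated, with a sign flip that makes full negative input turn the same way as positive.
; Mouse input drives controller yaw and pitch.
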(event `self.ReceiveBeginPlay`
  (`/Game/Blueprints/SC_HoverComponent.InitComponent` (`self.SC_HoverComponent1`) (`self.StaticMesh`))
  (`/Game/Blueprints/SC_HoverComponent.InitComponent` (`self.SC_HoverComponent2`) (`self.StaticMesh`))
  (`/Game/Blueprints/SC_HoverComponent.InitComponent` (`self.SC_HoverComponent3`) (`self.StaticMesh`))
  (`/Game/Blueprints/SC_HoverComponent.InitComponent` (`self.SC_HoverComponent4`) (`self.StaticMesh`)))

(event `InputAxis|MoveForward`
  (params (AxisValue :type "Float (single-precision)"))
  (bind _staticmesh (`self.StaticMesh`))
  (bind _canmove_ (`self.CheckIfCanMove`))
  (if _canmove_
    (`PrimitiveComponent.AddForce` _staticmesh (* (* (`SceneComponent.GetForwardVector` _staticmesh) (`self.ForwardForce`)) AxisValue) "None" true)))

(event `InputAxis|MoveRight`
  (params (AxisValue :type "Float (single-precision)"))
  (`PrimitiveComponent.AddTorqueInRadians` (`self.StaticMesh`) (`KismetMathLibrary.MakeVector` 0.0 0.0 (* (`KismetMathLibrary.SelectFloat` 1.0 -1.0 (not (== (stale `InputAxis|MoveForward` AxisValue) -1.0))) (* AxisValue (`self.Torque`)))) "None" true))

(event `InputAxis|MouseX`
  (params (AxisValue :type "Float (single-precision)"))
  (`self.AddControllerYawInput` AxisValue))

(event `InputAxis|MouseY`
  (params (AxisValue :type "Float (single-precision)"))
  (`self.AddControllerPitchInput` AxisValue))

(event `self.ReceiveTick`
  (params (DeltaSeconds :type "Float (single-precision)"))
  (`PrimitiveComponent.AddForce` (`self.StaticMesh`) (0.0 0.0 -10000.0) "None" false))

(fn `CheckIfCanMove`
  (returns (`CanMove?` :type Boolean))
  (if (or (`/Game/Blueprints/SC_HoverComponent.CanMove?` (`self.SC_HoverComponent1`)) (`/Game/Blueprints/SC_HoverComponent.CanMove?` (`self.SC_HoverComponent2`)) (`/Game/Blueprints/SC_HoverComponent.CanMove?` (`self.SC_HoverComponent3`)) (`/Game/Blueprints/SC_HoverComponent.CanMove?` (`self.SC_HoverComponent4`)))
    (return true)
    (else
      (return false))))

(fn `UserConstructionScript`)