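; Player controller for the wheelchair pawn that owns the HUD and shows notifications for the pawn's 180, 360 and 720 events.
; On BeginPlay it caches the player pawn as BP_Wheelchair, creates WBP_HUD and binds to those three pawn event dispatchers.
; Each handler passes its own enum value to the HUD's PlayNotification.
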(event `self.ReceiveBeginPlay`
  (bind _playerpawn (`self.PlayerPawn`))
  (`|ExecutionSequence`
    (:`then_0`
      (bind _asbp_wheelchair (cast `/Game/Blueprints/Actors/BP_Wheelchair` (`GameplayStatics.GetPlayerPawn` 0)))
      (set `self.PlayerPawn` _asbp_wheelchair)
      (bind _returnvalue (`|CreateWidget` "/Game/Widgets/WBP_HUD.WBP_HUD_C"))
      (bind _output_get (set `self.HUD` _returnvalue))
      (`UserWidget.AddToViewport` _output_get 0))
    (:`then_1`
      (add `/Game/Blueprints/Actors/BP_Wheelchair.180` _playerpawn (delegate `On180`))
      (add `/Game/Blueprints/Actors/BP_Wheelchair.360` _playerpawn (delegate `On360`))
      (add `/Game/Blueprints/Actors/BP_Wheelchair.720` _playerpawn (delegate `On720`)))))

(event `On180`
  (`/Game/Widgets/WBP_HUD.PlayNotification` (`self.HUD`) "NewEnumerator0"))

(event `On360`
  (`/Game/Widgets/WBP_HUD.PlayNotification` (`self.HUD`) "NewEnumerator1"))

(event `On720`
  (`/Game/Widgets/WBP_HUD.PlayNotification` (`self.HUD`) "NewEnumerator2"))

(fn `UserConstructionScript`)